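; Actor for the second right-thumb joint in the WaveVR natural hand tracking test, drawing that joint and its link to the next.
; Each Tick, a valid WaveVRHandJoint pose sets the static mesh's relative location and rotation.
; A beam particle then runs from this actor's location to the first R_Thumb_Joint3 actor, looked up every frame with GetAllActorsOfClass.
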(event `self.ReceiveTick`
  (params (DeltaSeconds :type "Float (single-precision)"))
  (bind _wavevrhandjoint (`self.WaveVRHandJoint`))
  (`|ExecutionSequence`
    (:`then_0`
      (bind _returnvalue (`WaveVRHandJointComponent.IsValidPose` _wavevrhandjoint))
      (if _returnvalue
        (bind _returnvalue_2 (`WaveVRHandJointComponent.GetLocation` _wavevrhandjoint))
        (bind _returnvalue_3 (`WaveVRHandJointComponent.GetRotation` _wavevrhandjoint))
        (`SceneComponent.K2_SetRelativeLocationAndRotation` (`self.StaticMeshComponent`) _returnvalue_2 _returnvalue_3 false false)))
    (:`then_1`
      (`ParticleSystemComponent.SetBeamSourcePoint` (`self.ParticleSystem`) 0 (`self.K2_GetActorLocation`) 0)
      (bind _outactors (`GameplayStatics.GetAllActorsOfClass` "/Game/VRTestApp/HandTracking/NaturalHand/Blueprints/Right_Hand/R_Thumb_Joint3.R_Thumb_Joint3_C"))
      (`ParticleSystemComponent.SetBeamTargetPoint` (`self.ParticleSystem`) 0 (`self.K2_GetActorLocation` (`|GetArrayItem` _outactors)) 0))))

(fn `UserConstructionScript`)