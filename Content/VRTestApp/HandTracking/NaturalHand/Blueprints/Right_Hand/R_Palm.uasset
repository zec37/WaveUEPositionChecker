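; Right-hand palm Blueprint for the natural hand tracking part of a VR test app, showing the tracked palm with a static mesh.
; Each tick, it reads the WaveVR hand joint and, when the pose is valid, applies its location and rotation to the mesh's relative transform.
; A counter periodically prints the right hand's tracking confidence as debug output, counting only valid-pose ticks.
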(event `self.ReceiveBeginPlay`)

(event `self.ReceiveTick`
  (params (DeltaSeconds :type "Float (single-precision)"))
  (bind _wavevrhandjoint (`self.WaveVRHandJoint`))
  (bind _returnvalue (`WaveVRHandJointComponent.IsValidPose` _wavevrhandjoint))
  (if _returnvalue
    (bind _returnvalue_2 (`WaveVRHandJointComponent.GetLocation` _wavevrhandjoint))
    (bind _returnvalue_3 (`WaveVRHandJointComponent.GetRotation` _wavevrhandjoint))
    (`SceneComponent.K2_SetRelativeLocationAndRotation` (`self.StaticMeshComponent`) _returnvalue_2 _returnvalue_3 false false)
    (bind _result (`/Engine/EditorBlueprintResources/StandardMacros.IncrementInt` (`self.counter`))
      (:`  `
        (if (>= _result 200)
          (set `self.counter` 0)
          (bind _returnvalue_4 (`WaveVRHandBPLibrary.GetHandConfidence` "Natural" "Right"))
          (`KismetSystemLibrary.PrintString` (`KismetStringLibrary.Concat_StrStr` "Right confidence: " (`KismetStringLibrary.Conv_DoubleToString` _returnvalue_4))))))))

(fn `UserConstructionScript`)