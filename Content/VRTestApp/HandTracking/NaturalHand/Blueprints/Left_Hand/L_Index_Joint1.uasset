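; Actor for the first left index finger joint in the Wave VR natural hand tracking test.
; Each tick, it moves its static mesh to the WaveVRHandJoint location when the pose is valid.
; It also updates a particle beam from its own actor location to the first L_Index_Joint2 actor, found by a per-tick GetAllActorsOfClass lookup, linking the two joints visually.
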(event `self.ReceiveTick`
  (params (DeltaSeconds :type "Float (single-precision)"))
  (bind _wavevrhandjoint (`self.WaveVRHandJoint`))
  (`|ExecutionSequence`
    (:`then_0`
      (bind _returnvalue (`WaveVRHandJointComponent.IsValidPose` _wavevrhandjoint))
      (if _returnvalue
        (bind _returnvalue_2 (`WaveVRHandJointComponent.GetLocation` _wavevrhandjoint))
        (`SceneComponent.K2_SetRelativeLocation` (`self.StaticMeshComponent`) _returnvalue_2 false false)))
    (:`then_1`
      (`ParticleSystemComponent.SetBeamSourcePoint` (`self.ParticleSystem`) 0 (`self.K2_GetActorLocation`) 0)
      (bind _outactors (`GameplayStatics.GetAllActorsOfClass` "/Game/VRTestApp/HandTracking/NaturalHand/Blueprints/Left_Hand/L_Index_Joint2.L_Index_Joint2_C"))
      (`ParticleSystemComponent.SetBeamTargetPoint` (`self.ParticleSystem`) 0 (`self.K2_GetActorLocation` (`|GetArrayItem` _outactors)) 0))))

(fn `UserConstructionScript`)