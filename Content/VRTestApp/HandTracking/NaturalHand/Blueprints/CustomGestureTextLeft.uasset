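; VR test display that shows the left hand's custom WaveVR gesture and motion details on a TextRender.
; On BeginPlay it binds to the left and dual custom gesture events, both of which store the gesture name under the same "Left(Custom):" label.
; Each Tick it polls the Natural tracker's left-hand motion, appending pinch strength, origin and direction or hold role and object type to that label.
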(event `self.ReceiveBeginPlay`
  (add `WaveVRHandGestureComponent.OnCustomGestureBp_Left` (`self.WaveVRHandGesture`) (delegate `LeftCustomEvent`))
  (add `WaveVRHandGestureComponent.OnCustomGestureBp_Dual` (`self.WaveVRHandGesture`) (delegate `DualCustomEvent`)))

(event `LeftCustomEvent`
  (params (gesture :type String))
  (set `self.GestureText` (`KismetStringLibrary.Concat_StrStr` "Left(Custom): " gesture)))

(event `DualCustomEvent`
  (params (gesture :type String))
  (set `self.GestureText` (`KismetStringLibrary.Concat_StrStr` "Left(Custom): " gesture)))

(event `self.ReceiveTick`
  (params (DeltaSeconds :type "Float (single-precision)"))
  (bind _returnvalue (`WaveVRHandBPLibrary.GetHandMotion` "Natural" "Left"))
  (switch `EWaveVRHandMotion` _returnvalue
    (:`Invalid`
      (`TextRenderComponent.K2_SetText` (`self.TextRender`) (`KismetTextLibrary.Conv_StringToText` (`self.GestureText`))))
    (:`Pinch`
      (bind _returnvalue_2 (`WaveVRHandBPLibrary.GetHandPinchStrength` "Natural" "Left"))
      (bind _returnvalue_3 (`WaveVRHandBPLibrary.GetHandPinchOrigin` "Natural" "Left"))
      (bind _returnvalue_4 (`WaveVRHandBPLibrary.GetHandPinchDirection` "Natural" "Left"))
      (`TextRenderComponent.K2_SetText` (`self.TextRender`) (`KismetTextLibrary.Conv_StringToText` (`KismetStringLibrary.Concat_StrStr` (`KismetStringLibrary.Concat_StrStr` (`KismetStringLibrary.Concat_StrStr` (`self.GestureText`) (`KismetStringLibrary.Concat_StrStr` ", pinch strength: " (`KismetStringLibrary.Conv_DoubleToString` _returnvalue_2))) (`KismetStringLibrary.Concat_StrStr` ", origin: " (`KismetStringLibrary.Conv_VectorToString` _returnvalue_3))) (`KismetStringLibrary.Concat_StrStr` ", direction: " (`KismetStringLibrary.Conv_VectorToString` _returnvalue_4))))))
    (:`Hold`
      (bind _returnvalue_5 (`WaveVRHandBPLibrary.GetHandHoldRole` "Natural" "Left"))
      (bind _returnvalue_6 (`WaveVRHandBPLibrary.GetHandHoldType` "Natural" "Left"))
      (`TextRenderComponent.K2_SetText` (`self.TextRender`) (`KismetTextLibrary.Conv_StringToText` (`KismetStringLibrary.Concat_StrStr` (`KismetStringLibrary.Concat_StrStr` (`self.GestureText`) (`KismetStringLibrary.Concat_StrStr` ", hold role: " (`|GetEnumeratorNameAsString` _returnvalue_5))) (`KismetStringLibrary.Concat_StrStr` ", object: " (`|GetEnumeratorNameAsString` _returnvalue_6))))))))

(fn `UserConstructionScript`)