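; BP_Cube is a VR test cube that responds to raycast-style interaction events by showing the event name on its surface and rotating while hovered.
; Click, enter and exit set the text, then, as on BeginPlay, create a new canvas render target and trigger an update.
; The update callback draws the text over a black background and feeds the target into a new dynamic M_Rock material instance on the mesh.
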(event `WaveVRInteractInterface.OnClick`
  (params (caller :type "Actor Object Reference"))
  (set `self.CubeText` "Click")
  ;[1 1 1] New texture
  (bind _returnvalue (`CanvasRenderTarget2D.CreateCanvasRenderTarget2D` "/Script/Engine.CanvasRenderTarget2D" :!label _label))
  (bind _output_get (set `self.CustomTexture_0` _returnvalue))
  (add `CanvasRenderTarget2D.OnCanvasRenderTargetUpdate` _output_get (delegate `CustomEvent_0`))
  (`CanvasRenderTarget2D.UpdateResource` _output_get))

(event `WaveVRInteractInterface.OnEnter`
  (params (caller :type "Actor Object Reference"))
  (set `self.CubeText` "Enter")
  (goto _label))

(event `WaveVRInteractInterface.OnExit`
  (params (caller :type "Actor Object Reference"))
  (set `self.CubeText` "Exit")
  (goto _label))

(event `self.ReceiveBeginPlay`
  (goto _label))

(event `CustomEvent_0`
  (params (Canvas :type "Canvas Object Reference") (Width :type Integer) (Height :type Integer))
  (bind _staticmeshcomponent (`self.StaticMeshComponent`))
  ;[1 1 1] New texture
  (bind _output_get (set `self.Canvas_0` Canvas))
  (`Canvas.K2_DrawTexture` _output_get "/Engine/EngineResources/Black_Low.Black" (0.0 0.0) (`KismetMathLibrary.MakeVector2D` (`KismetMathLibrary.Conv_IntToDouble` Width) (`KismetMathLibrary.Conv_IntToDouble` Height)) (0.0 0.0) (1.0 1.0) (struct :`R` 1.0 :`G` 1.0 :`B` 1.0 :`A` 1.0) "BLEND_Opaque" 0.0 (0.5 0.5))
  (`Canvas.K2_DrawText` _output_get "/Game/VRTestApp/Raycast/Materials/FontInteraction.FontInteraction" (`self.CubeText`) (200.0 400.0) (10.0 10.0) (struct :`R` 1.0 :`G` 1.0 :`B` 1.0 :`A` 1.0) 0.0 (struct :`A` 1.0) (1.0 1.0) false false false (struct :`A` 1.0))
  (bind _returnvalue (`PrimitiveComponent.CreateDynamicMaterialInstance` _staticmeshcomponent 0 "/Game/VRTestApp/Resources/Materials/M_Rock.M_Rock" "None"))
  (`PrimitiveComponent.SetMaterial` _staticmeshcomponent 0 _returnvalue)
  ;[1 1 1] "TP2D" in MatInteraction
  (`MaterialInstanceDynamic.SetTextureParameterValue` _returnvalue "TP2D" (`self.CustomTexture_0`)))

(event `WaveVRInteractInterface.OnHover`
  (params (caller :type "Actor Object Reference"))
  (`SceneComponent.K2_AddRelativeRotation` (`self.StaticMeshComponent`) (struct :`Yaw` 1.0) false false))

(fn `UserConstructionScript`)