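; VR test Blueprint that displays which button is pressed on a given tracker through a text render component.
; Every Tick it resets the text to a "Press: N/A" default, then polls each entry in the Buttons array for the configured TrackerID.
; A pressed button replaces the default with its enum name, so the last pressed one in the array wins.
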(event `self.ReceiveTick`
  (params (DeltaSeconds :type "Float (single-precision)"))
  (set `self.ResultText` (`KismetStringLibrary.Concat_StrStr` (`self.TrackerText`) "Press: N/A"))
  (for _array_element (`self.Buttons`)
    (bind _returnvalue (`WaveVRTrackerBPLibrary.IsTrackerButtonPressed` (`self.TrackerID`) _array_element))
    (if _returnvalue
      (set `self.ResultText` (`KismetStringLibrary.Concat_StrStr` (`self.TrackerText`) (`KismetStringLibrary.Concat_StrStr` "Press: " (`|GetEnumeratorNameAsString` _array_element)))))
    (`TextRenderComponent.K2_SetText` (`self.TextRender`) (`KismetTextLibrary.Conv_StringToText` (`self.ResultText`)))))

(fn `UserConstructionScript`)