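; Debug text display in the VR test app's Bracelet folder that shows the live connection status of a VR tracker.
; Every Tick it queries whether its Tracker is connected and writes the TrackerText label plus that status to a TextRender.
; When the tracker is connected, it also appends the tracker's degree-of-freedom mode.
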(event `self.ReceiveTick`
  (params (DeltaSeconds :type "Float (single-precision)"))
  (bind _tracker (`self.Tracker`))
  (bind _returnvalue (`WaveVRTrackerBPLibrary.IsTrackerConnected` _tracker))
  (if _returnvalue
    (bind _dof (`WaveVRTrackerBPLibrary.GetTrackerDegreeOfFreedom` _tracker))
    (bind _returnvalue_2 (`KismetStringLibrary.Concat_StrStr` (`KismetStringLibrary.Concat_StrStr` (`self.TrackerText`) " ") (`KismetStringLibrary.Concat_StrStr` "Connect: " (`KismetStringLibrary.Conv_BoolToString` _returnvalue))))
    (`TextRenderComponent.K2_SetText` (`self.TextRender`) (`KismetTextLibrary.Conv_StringToText` (`KismetStringLibrary.Concat_StrStr` (`KismetStringLibrary.Concat_StrStr` _returnvalue_2 ", ") (`|GetEnumeratorNameAsString` _dof))))
    (else
      (`TextRenderComponent.K2_SetText` (`self.TextRender`) (`KismetTextLibrary.Conv_StringToText` _returnvalue_2)))))

(fn `UserConstructionScript`)