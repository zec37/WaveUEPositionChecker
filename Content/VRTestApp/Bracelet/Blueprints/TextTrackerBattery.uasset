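; TextTrackerBattery is a Blueprint in the VR test app's Bracelet folder that displays a tracker's battery level as text.
; Every Tick it reads the battery life for its TrackerID, multiplies it by 100 and appends it to the TrackerText label as a percentage.
; The resulting string is written to the TextRender component, while BeginPlay and the construction script do nothing.
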(event `self.ReceiveTick`
  (params (DeltaSeconds :type "Float (single-precision)"))
  (bind _returnvalue (`WaveVRTrackerBPLibrary.GetTrackerBatteryLife` (`self.TrackerID`)))
  (`TextRenderComponent.K2_SetText` (`self.TextRender`) (`KismetTextLibrary.Conv_StringToText` (`KismetStringLibrary.Concat_StrStr` (`KismetStringLibrary.Concat_StrStr` (`KismetStringLibrary.Concat_StrStr` (`self.TrackerText`) "Battery: ") (`KismetStringLibrary.Conv_DoubleToString` (* 100 _returnvalue))) "%"))))

(fn `UserConstructionScript`)