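; BraceletTracker5 is an actor in a VR bracelet test app that shows the live pose of Tracker 5 with a static mesh.
; Each Tick on non-Windows platforms, it moves the mesh to the tracker position plus the BraceletPawn's CameraHeight and a LocOffset, using the tracker's quaternion for rotation.
; The mesh hides whenever the tracker pose is invalid.
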(event `self.ReceiveTick`
  (params (DeltaSeconds :type "Float (single-precision)"))
  (if (not (`KismetStringLibrary.EqualEqual_StrStr` (`GameplayStatics.GetPlatformName`) "Windows"))
    (bind _asbracelet_pawn (cast `/Game/VRTestApp/Bracelet/BraceletPawn` (`GameplayStatics.GetPlayerPawn` 0)))
    (bind _outposition (`WaveVRTrackerBPLibrary.GetTrackerPosition` "Tracker5"))
    (bind _outorientation (`WaveVRTrackerBPLibrary.GetTrackerRotation` "Tracker5"))
    (`SceneComponent.K2_SetRelativeLocationAndRotation` (`self.StaticMeshComponent`) (+ (+ _outposition (`/Game/VRTestApp/Bracelet/BraceletPawn.CameraHeight` _asbracelet_pawn)) (`self.LocOffset`)) (`KismetMathLibrary.Quat_Rotator` _outorientation) false false)
    (bind _returnvalue (`WaveVRTrackerBPLibrary.IsTrackerPoseValid` "Tracker5"))
    (`SceneComponent.SetHiddenInGame` (`self.StaticMeshComponent`) (not _returnvalue) false)))

(fn `UserConstructionScript`)