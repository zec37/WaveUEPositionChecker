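; VR test app Blueprint in the Bracelet folder that displays a tracker's extended data as on-screen text for inspection.
; Each Tick it reads the extended data array with its timestamp and concatenates the elements, without separators, into a string.
; A TextRender shows that string with the tracker label and timestamp, then the buffer is cleared.
; An alternative read without timestamp is left unconnected to any event.
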(event `self.ReceiveTick`
  (params (DeltaSeconds :type "Float (single-precision)"))
  (bind (_validsize _timestamp _returnvalue) (`WaveVRTrackerBPLibrary.GetTrackerExtendedDataTimestamp` (`self.Tracker`)))
  (for _array_element _returnvalue
    (bind _output_get (set `self.result` (`KismetStringLibrary.Concat_StrStr` (stale _output_get) (`KismetStringLibrary.Conv_IntToString` _array_element)))))
  (`TextRenderComponent.K2_SetText` (`self.TextRender`) (`KismetTextLibrary.Conv_StringToText` (`KismetStringLibrary.Concat_StrStr` (`KismetStringLibrary.Concat_StrStr` (`KismetStringLibrary.Concat_StrStr` (`KismetStringLibrary.Concat_StrStr` (`self.TrackerText`) " Ext: ") (`self.result`)) ", ") (`KismetStringLibrary.Conv_IntToString` _timestamp))))
  (set `self.result` ""))

(fn `UserConstructionScript`)