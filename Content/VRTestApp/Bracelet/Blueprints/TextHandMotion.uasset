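; Debug text actor for the VR bracelet test app that displays the current motion of both hands.
; Each tick it queries the hand motion for the left and right hands using the Natural tracker.
; It converts both motion enums to strings, joins them with the left and right hand labels, and writes the result to a TextRender component.
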(event `self.ReceiveTick`
  (params (DeltaSeconds :type "Float (single-precision)"))
  (`|ExecutionSequence`
    (:`then_0`
      (bind _returnvalue (`WaveVRHandBPLibrary.GetHandMotion` "Natural" "Left")))
    (:`then_1`
      (bind _returnvalue_2 (`WaveVRHandBPLibrary.GetHandMotion` "Natural" "Right")))
    (:`then_4`
      (`TextRenderComponent.K2_SetText` (`self.TextRender`) (`KismetTextLibrary.Conv_StringToText` (`KismetStringLibrary.Concat_StrStr` (`KismetStringLibrary.Concat_StrStr` (`KismetStringLibrary.Concat_StrStr` "Motion: " (`KismetStringLibrary.Concat_StrStr` (`self.LeftHand`) (`|GetEnumeratorNameAsString` _returnvalue))) ", ") (`KismetStringLibrary.Concat_StrStr` (`self.RightHand`) (`|GetEnumeratorNameAsString` _returnvalue_2))))))))

(fn `UserConstructionScript`)