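; Debug text display in the VR test app that shows which buttons on a bracelet tracker are currently touched.
; Each Tick it rebuilds a string from the tracker label, looping over the Buttons array and querying touch state and axis for the configured TrackerID.
; Touched buttons are appended by enum name with their axis value, and the result is written to a TextRender.
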(event `self.ReceiveTick`
  (params (DeltaSeconds :type "Float (single-precision)"))
  (bind _trackerid (`self.TrackerID`))
  (set `self.ResultText` (`KismetStringLibrary.Concat_StrStr` (`self.TrackerText`) "Touch: "))
  (for _array_element (`self.Buttons`)
    (bind _returnvalue (`WaveVRTrackerBPLibrary.IsTrackerButtonTouched` _trackerid _array_element))
    (bind _returnvalue_2 (`WaveVRTrackerBPLibrary.GetTrackerButtonAxis` _trackerid _array_element))
    (bind _output_get (set `self.axis` _returnvalue_2))
    (if _returnvalue
      (set `self.ResultText` (`KismetStringLibrary.Concat_StrStr` (`KismetStringLibrary.Concat_StrStr` (`KismetStringLibrary.Concat_StrStr` (`KismetStringLibrary.Concat_StrStr` (`self.ResultText`) (`|GetEnumeratorNameAsString` _array_element)) " \n") ", ") (`KismetStringLibrary.Conv_Vector2dToString` _output_get))))
    (`TextRenderComponent.K2_SetText` (`self.TextRender`) (`KismetTextLibrary.Conv_StringToText` (`self.ResultText`)))))

(fn `UserConstructionScript`)