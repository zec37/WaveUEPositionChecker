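; TextTrackerName is a Blueprint in the VR test app's Bracelet folder that displays the device name of one tracker, chosen by TrackerID, on a text render component.
; Every Tick it queries that tracker's device name and the currently focused tracker, then rewrites the text as TrackerText plus the name.
; A ",focused" suffix is added when the focus query succeeds and its ID matches TrackerID.
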(event `self.ReceiveTick`
  (params (DeltaSeconds :type "Float (single-precision)"))
  (bind _textrender (`self.TextRender`))
  (bind _trackerid (`self.TrackerID`))
  (bind _devicename (`WaveVRTrackerBPLibrary.GetTrackerDeviceName` _trackerid))
  (bind (_trackerid_2 _returnvalue) (`WaveVRTrackerBPLibrary.GetFocusedTracker`))
  (if _returnvalue
    (if (`|EnumEquality` _trackerid_2 _trackerid)
      (bind _returnvalue_2 (`KismetStringLibrary.Concat_StrStr` (`self.TrackerText`) _devicename))
      (`TextRenderComponent.K2_SetText` _textrender (`KismetTextLibrary.Conv_StringToText` (`KismetStringLibrary.Concat_StrStr` _returnvalue_2 ",focused")))
      (else
        (`TextRenderComponent.K2_SetText` _textrender (`KismetTextLibrary.Conv_StringToText` _returnvalue_2) :!label _label)))
    (else
      (goto _label))))

(fn `UserConstructionScript`)