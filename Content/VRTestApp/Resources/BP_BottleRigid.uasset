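; Physics bottle in the VR test app that plays impact sounds matching how hard and at what tilt it hits.
; Tick caches mesh velocity, so Hit can use the larger of pre- and post-impact speed.
; Strong hits pick upright, side, cap or force-tiered sounds from tilt and speed, with speed-scaled volume.
; Weaker hits play water sloshing; DoOnce and Delay cooldowns throttle both kinds.
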(event `self.ReceiveTick`
  (params (DeltaSeconds :type "Float (single-precision)"))
  (set `self.LastFrameVelocity` (`SceneComponent.GetComponentVelocity` (`self.StaticMeshComponent`))))

(event `self.ReceiveHit`
  (params (MyComp :type "PrimitiveComponent Object Reference") (Other :type "Actor Object Reference") (OtherComp :type "PrimitiveComponent Object Reference") (bSelfMoved :type Boolean) (HitLocation :type "Vector Structure") (HitNormal :type "Vector Structure") (NormalImpulse :type "Vector Structure") (Hit :type "HitResult Structure (by ref)"))
  (bind _returnvalue (`KismetMathLibrary.FMax` (`KismetMathLibrary.VSize` (`SceneComponent.GetComponentVelocity` MyComp)) (`KismetMathLibrary.VSize` (`self.LastFrameVelocity`))))
  (bind _returnvalue_2 (`KismetMathLibrary.DegAcos` (`KismetMathLibrary.Dot_VectorVector` (`KismetMathLibrary.GetUpVector` (`SceneComponent.K2_GetComponentRotation` MyComp)) (0.0 0.0 1.0))))
  (bind _returnvalue_3 (< _returnvalue_2 10.0))
  (bind _returnvalue_4 (+ (- (* (/ (`KismetMathLibrary.FClamp` _returnvalue 0.0 800.0) 100.0) 0.4) 0.2) 1.0))
  (if (> _returnvalue 200.0)
    (`/Engine/EditorBlueprintResources/StandardMacros.DoOnce` false :!label _label
      (:`Completed`
        ;[1 1 1] Hit Angle 10~80
        (if (and (< _returnvalue_2 80.0) (not _returnvalue_3))
          ;[1 1 1] Hit Force
          (if (< _returnvalue 400.0)
            (`GameplayStatics.PlaySoundAtLocation` (`self.SoundHitSlightForce`) HitLocation (struct) _returnvalue_4 1.0 0.0 "/Game/VRTestApp/Resources/Sound/BottleSoundAttenuation.BottleSoundAttenuation" "/Game/VRTestApp/Resources/Sound/BottleSoundConcurrency.BottleSoundConcurrency" null)
            (elif (< _returnvalue 600.0)
              (`GameplayStatics.PlaySoundAtLocation` (`self.SoundHitMiddleForce`) HitLocation (struct) _returnvalue_4 1.0 0.0 "/Game/VRTestApp/Resources/Sound/BottleSoundAttenuation.BottleSoundAttenuation" "/Game/VRTestApp/Resources/Sound/BottleSoundConcurrency.BottleSoundConcurrency" null)
              (else
                (`GameplayStatics.PlaySoundAtLocation` (`self.SoundHitStraight`) HitLocation (struct) _returnvalue_4 1.0 0.0 "/Game/VRTestApp/Resources/Sound/BottleSoundAttenuation.BottleSoundAttenuation" "/Game/VRTestApp/Resources/Sound/BottleSoundConcurrency.BottleSoundConcurrency" null :!label _label_2))))
          (else
            ;[1 1 1] Hit Angle < 10
            (if _returnvalue_3
              (goto _label_2)
              (elif (> _returnvalue_2 135.0)
                (`GameplayStatics.PlaySoundAtLocation` (`self.SoundHitOnCap`) HitLocation (struct) _returnvalue_4 1.0 0.0 "/Game/VRTestApp/Resources/Sound/BottleSoundAttenuation.BottleSoundAttenuation" "/Game/VRTestApp/Resources/Sound/BottleSoundConcurrency.BottleSoundConcurrency" null)
                (else
                  (`GameplayStatics.PlaySoundAtLocation` (`self.SoundHitSide`) HitLocation (struct) _returnvalue_4 1.0 0.0 "/Game/VRTestApp/Resources/Sound/BottleSoundAttenuation.BottleSoundAttenuation" "/Game/VRTestApp/Resources/Sound/BottleSoundConcurrency.BottleSoundConcurrency" null))))))
        (`KismetSystemLibrary.Delay` 0.4)
        (goto _label :!via `Reset`)))
    (elif (> _returnvalue 40.0)
      (`/Engine/EditorBlueprintResources/StandardMacros.DoOnce` false :!label _label_3
        (:`Completed`
          (`GameplayStatics.PlaySoundAtLocation` (`self.SoundWaterFlowInBottle`) HitLocation (struct) 1.0 1.0 0.0 "/Game/VRTestApp/Resources/Sound/BottleSoundAttenuation.BottleSoundAttenuation" "/Game/VRTestApp/Resources/Sound/BottleSoundConcurrency.BottleSoundConcurrency" null)
          (`KismetSystemLibrary.Delay` 2.0)
          (goto _label_3 :!via `Reset`))))))

(fn `UserConstructionScript`)